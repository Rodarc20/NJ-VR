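; VR controller-driven Blueprint for a node-and-edge graph visualization that lets the player move, rotate, scale and inspect it.
; Input actions set a mode (all, node, branch, area, none) and a task; Tick, Select press and Select release dispatch on that pair.
; Right-controller line traces find nodes, and a guide node anchors translation and branch rotation, with debug lines as lasers.
; Holding both grips scales the graph from the distance between controllers.
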(event EventBeginPlay
  (bind _asvrpawn_2vrv_bp (Utilities|Casting|CastToVRPawn2VRV_BP (Game|Player|GetPlayerPawn 0)))
  (Variables|Default|SetRightController (Variables|/Game/ControllerSetup/VRPawn2VRV_BP.VRPawn2VRV_BP_C|GetMotionControllerRight _asvrpawn_2vrv_bp))
  (Variables|Default|SetLeftController (Variables|/Game/ControllerSetup/VRPawn2VRV_BP.VRPawn2VRV_BP_C|GetMotionControllerLeft _asvrpawn_2vrv_bp))
  (Variables|/Game/ControllerSetup/VRPawn2VRV_BP.VRPawn2VRV_BP_C|SetVisualization _asvrpawn_2vrv_bp self)
  (Variables|Default|SetInteraction (Variables|/Game/ControllerSetup/VRPawn2VRV_BP.VRPawn2VRV_BP_C|GetInteraction _asvrpawn_2vrv_bp))
  (Variables|Default|SetDocument (Variables|/Game/ControllerSetup/VRPawn2VRV_BP.VRPawn2VRV_BP_C|GetDocument _asvrpawn_2vrv_bp)))

(event EventTick
  (params (DeltaSeconds :type Float%20%28single-precision%29))
  (bind _rightcontroller (Variables|Default|GetRightController))
  (bind _rightcontroller_2 (Variables|Default|GetRightController))
  (bind _distancialaser (Variables|Default|GetDistanciaLaser))
  (bind _rightcontroller_3 (Variables|Default|GetRightController))
  (bind _returnvalue (Math|Vector|GetForwardVector _rightcontroller_3))
  (bind _returnvalue_2 (Transformation|GetWorldLocation _rightcontroller_3))
  (bind _returnvalue_3 (Transformation|GetWorldLocation _rightcontroller))
  (bind _returnvalue_4 (Math|Vector|GetForwardVector _rightcontroller))
  (bind _returnvalue_5 (Transformation|GetWorldLocation _rightcontroller_2))
  (bind _returnvalue_6 (Math|Vector|GetForwardVector _rightcontroller_2))
  (bind _returnvalue_7 (* _returnvalue _distancialaser))
  (bind _returnvalue_8 (* _returnvalue_4 1e+03))
  (bind _returnvalue_9 (* _returnvalue_6 1e+03))
  (bind _returnvalue_10 (+ _returnvalue_3 _returnvalue_8))
  (bind _returnvalue_11 (+ _returnvalue_5 _returnvalue_9))
  (bind _returnvalue_12 (+ _returnvalue_2 _returnvalue_7))
  (if (Variables|Default|GetbCalcularEscala)
    (Class|VRVisualization|CalcularEscalaTemporal)
    (Class|VRVisualization|AplicarEscala (Variables|Default|GetEscalaTemp)))
  (bind _returnvalue_13 (Class|VRVisualization|GetVisualizationMode))
  ;[1 1 1] seleccionar el modo, sin area tengo 4, no selecciona es la visualizacion completa
  (switch Utilities|FlowControl|Switch|SwitchonEVRVisualizationMode _returnvalue_13
    (:EAll
      ;[1 1 1] Todo
      (bind _returnvalue_14 (Class|VRVisualization|GetVisualizationTask))
      (switch Utilities|FlowControl|Switch|SwitchonEVRVisualizationTask _returnvalue_14
        (:ETraslationTask
          (if (Variables|Default|GetbNodoGuia)
            ;[0.155 0.155 0.155] Buscar un punto en los limites de la visualizacion don de trasladar los nodos, este puedesta cosa puede ser reemplazada por calculos
            (bind (_outhit _returnvalue_15) (Collision|LineTraceForObjects _returnvalue_5 _returnvalue_11 (Utilities|Array|MakeArray "ObjectTypeQuery9") false 0 "None" false :!label _label))
            (bind _output_get (Variables|Default|SetbHitBoard _returnvalue_15))
            (Variables|Default|SetHitActor (.HitActor (Collision|BreakHitResult _outhit)))
            (if _output_get
              (Rendering|Debug|DrawDebugLine _returnvalue_5 (.ImpactPoint (Collision|BreakHitResult _outhit)) "(R=0.000000,G=0.475000,B=0.018212,A=1.000000)" 0.0 0.5)
              (Class|VRVisualization|AplicarTraslacion (- (.ImpactPoint (Collision|BreakHitResult _outhit)) (Transformation|GetActorLocation (Variables|Default|GetNodoGuia))))
              (else
                (Rendering|Debug|DrawDebugLine _returnvalue_5 _returnvalue_11 "(R=0.905000,G=0.000000,B=0.000000,A=1.000000)" 0.0 0.5)))
            (else
              (Class|VRVisualization|BuscandoNodoConLaser :!label _label_2))))
        (:ENoTask
          (goto _label_2))))
    (:ENode
      ;[1 1 1] Nodo
      (bind _returnvalue_16 (Class|VRVisualization|GetVisualizationTask))
      ;;[1 1 1] la tarea seleccionar esta impicata en todos los otrso mdos
      (switch Utilities|FlowControl|Switch|SwitchonEVRVisualizationTask _returnvalue_16
        (:ETraslationTask
          (if (Variables|Default|GetbNodoGuia)
            (goto _label)
            (else
              _)))
        (:EVisualizationTask
          _)
        (:ENoTask
          _))
      (Class|VRVisualization|BuscandoNodoConLaser))
    (:EBranch
      ;[1 1 1] Rama
      (bind _returnvalue_17 (Class|VRVisualization|GetVisualizationTask))
      (switch Utilities|FlowControl|Switch|SwitchonEVRVisualizationTask _returnvalue_17
        (:ETraslationTask
          (if (Variables|Default|GetbNodoGuia)
            (Class|NJ3DVRVisualization|TraslacionConNodoGuia)
            (else
              (Class|VRVisualization|BuscandoNodoConLaser :!label _label_3))))
        (:ERotationTask
          (if (Variables|Default|GetbNodoGuia)
            ;[0.155 0.155 0.155] Tarea Rotar Rama
            (bind (_outhit_2 _returnvalue_18) (Collision|LineTraceForObjects _returnvalue_3 _returnvalue_10 (Utilities|Array|MakeArray "ObjectTypeQuery9") false 0 "None" false))
            (bind _output_get_2 (Variables|Default|SetbHitBoard _returnvalue_18))
            (Variables|Default|SetHitActor (.HitActor (Collision|BreakHitResult _outhit_2)))
            (if _output_get_2
              (Rendering|Debug|DrawDebugLine _returnvalue_3 (.ImpactPoint (Collision|BreakHitResult _outhit_2)) "(R=0.000000,G=0.475000,B=0.018212,A=1.000000)" 0.0 0.5)
              (Class|VRVisualization|AplicarRotacionRelativaANodo (Variables|Default|GetNodoGuia) (.ImpactPoint (Collision|BreakHitResult _outhit_2)))
              (else
                (Rendering|Debug|DrawDebugLine _returnvalue_3 _returnvalue_10 "(R=0.905000,G=0.000000,B=0.000000,A=1.000000)" 0.0 0.5)))
            (else
              (goto _label_3))))
        (:ENoTask
          (goto _label_3))))
    (:ENoMode
      ;[1 1 1] Visualización, la tarea visualizacion solo deberia marcar dentro del menu
      (bind _returnvalue_19 (Class|VRVisualization|GetVisualizationTask))
      (switch Utilities|FlowControl|Switch|SwitchonEVRVisualizationTask _returnvalue_19
        (:ETraslationTask
          (if (Variables|Default|GetbNodoGuia)
            (Transformation|SetActorLocation (+ _returnvalue_12 (Variables|Default|GetOffsetToPointLaser)) false false)
            (Rendering|Debug|DrawDebugLine _returnvalue_2 _returnvalue_12 "(R=0.222584,G=0.000000,B=0.300000,A=1.000000)" 0.0 0.5)
            (else
              (Class|VRVisualization|BuscandoNodoConLaser :!label _label_4))))
        (:ERotationTask
          (if (Variables|Default|GetRotar)
            (Class|VRVisualization|RotarVisualizacion)
            (goto _label_4)
            (else
              (goto _label_4))))
        (:EVisualizationTask
          (goto _label_4))
        (:ENoTask
          (goto _label_4))))))

(event Input|ActionEvents|InputActionModeAll
  (params (Key :type Key%20Structure))
  ;[0.155 0.155 0.155] Visualizations Modes
  (:Pressed
    (Variables|Default|SetCurrentVisualizationMode "EAll")
    (Development|PrintText "Todo" true true "(R=0.000000,G=0.056297,B=1.000000,A=1.000000)" 5.0)))

(event Input|ActionEvents|InputActionModeIndividual
  (params (Key :type Key%20Structure))
  ;[0.155 0.155 0.155] Visualizations Modes
  (:Pressed
    ;;[1 1 1] COmo la variable es de esta clase, puedo modificarla directamente
    (Variables|Default|SetCurrentVisualizationMode "ENode")
    (Development|PrintText "Nodo por nodo" true true "(R=0.000000,G=0.056297,B=1.000000,A=1.000000)" 5.0)))

(event Input|ActionEvents|InputActionModeBranch
  (params (Key :type Key%20Structure))
  ;[0.155 0.155 0.155] Visualizations Modes
  (:Pressed
    (Variables|Default|SetCurrentVisualizationMode "EBranch")
    (Development|PrintText "Rama" true true "(R=0.000000,G=0.056297,B=1.000000,A=1.000000)" 5.0)))

(event Input|ActionEvents|InputActionModeArea
  (params (Key :type Key%20Structure))
  ;[0.155 0.155 0.155] Visualizations Modes
  (:Pressed
    ;;[1 1 1] pero lo correcto seria usar el setter
    (Class|VRVisualization|SetVisualizationMode "EArea")
    (Development|PrintText "Area" true true "(R=0.000000,G=0.056297,B=1.000000,A=1.000000)" 5.0)))

(event Input|ActionEvents|InputActionModeNone
  (params (Key :type Key%20Structure))
  ;[0.155 0.155 0.155] Visualizations Modes
  (:Pressed
    (Class|VRVisualization|SetVisualizationMode "ENoMode")
    (Development|PrintText "Ninguno" true true "(R=0.000000,G=0.056297,B=1.000000,A=1.000000)" 5.0)
    ;;[1 1 1] EStos al no requerir dar click en algun nodo, automaticamente edeben ser ejecutados al entrar en ese modo
    (Class|VRVisualization|DeseleccionarTodo)))

(event Input|ActionEvents|InputActionSostenerDerecha
  (params (Key :type Key%20Structure))
  ;[0.055 0.055 0.055] Escala
  (:Pressed
    (Variables|Default|SetbGripDerecho true)
    (if (Variables|Default|GetbGripIzquierdo)
      (Variables|Default|SetbCalcularEscala true)
      (Variables|Default|SetDistanciaInicialControles (Math|Vector|VectorLength (- (Transformation|GetWorldLocation (Variables|Default|GetRightController)) (Transformation|GetWorldLocation (Variables|Default|GetLeftController)))))))
  (:Released
    (Variables|Default|SetbGripDerecho false)
    (Variables|Default|SetbCalcularEscala false)
    (bind _output_get (Variables|Default|SetEscala (Variables|Default|GetEscalaTemp)))
    (Class|VRVisualization|AplicarEscala _output_get)))

(event Input|ActionEvents|InputActionSostenerIzquierda
  (params (Key :type Key%20Structure))
  ;[0.055 0.055 0.055] Escala
  (:Pressed
    (Variables|Default|SetbGripIzquierdo true)
    (if (Variables|Default|GetbGripDerecho)
      (Variables|Default|SetbCalcularEscala true)
      (Variables|Default|SetDistanciaInicialControles (Math|Vector|VectorLength (- (Transformation|GetWorldLocation (Variables|Default|GetRightController)) (Transformation|GetWorldLocation (Variables|Default|GetLeftController)))))))
  (:Released
    (Variables|Default|SetbGripIzquierdo false)
    (Variables|Default|SetbCalcularEscala false)
    (bind _output_get (Variables|Default|SetEscala (Variables|Default|GetEscalaTemp)))
    (Class|VRVisualization|AplicarEscala _output_get)))

(event Input|ActionEvents|InputActionSelect
  (params (Key :type Key%20Structure))
  (bind _hitnodo (Variables|Default|GetHitNodo))
  (:Pressed
    (bind _returnvalue (Class|VRVisualization|GetVisualizationMode))
    (switch Utilities|FlowControl|Switch|SwitchonEVRVisualizationMode _returnvalue
      (:EAll
        ;[1 1 1] Todo
        (bind _returnvalue_2 (Class|VRVisualization|GetVisualizationTask))
        (switch Utilities|FlowControl|Switch|SwitchonEVRVisualizationTask _returnvalue_2
          (:ETraslationTask
            (Class|VRVisualization|TrasladarTodoPressed))))
      (:ENode
        ;[1 1 1] Nodo
        (bind _returnvalue_3 (Class|VRVisualization|GetVisualizationTask))
        (switch Utilities|FlowControl|Switch|SwitchonEVRVisualizationTask _returnvalue_3
          (:ETraslationTask
            (Class|VRVisualization|TrasladarNodoPressed))
          (:EVisualizationTask
            (Class|VRVisualization|VisualizarNodoPressed)
            (if (Variables|Default|GetbHitNodo)
              ;[1 1 1] VisualizarNodoPressed
              (bind _ascontenido_nodo (Utilities|Casting|CastToContenidoNodo (UserInterface|GetUserWidgetObject (Variables|/Script/NJVR.Nodo|GetContenido _hitnodo))))
              (bind _output_get (Variables|/Game/Visualization/Blueprints/Menu/ContenidoNodo.ContenidoNodo_C|SetNodo _ascontenido_nodo _hitnodo))
              (bind _returnvalue_4 (Class|VRVisualization|ObtenerContenidoNodo _output_get))
              (Default|CambiarTexto _ascontenido_nodo (Utilities|Text|ToText(String) _returnvalue_4))
              (Class|Nodo|MostrarContenido _hitnodo)))))
      (:EBranch
        ;[1 1 1] Rama
        (bind _returnvalue_5 (Class|VRVisualization|GetVisualizationTask))
        (switch Utilities|FlowControl|Switch|SwitchonEVRVisualizationTask _returnvalue_5
          (:ETraslationTask
            (Class|NJ3DVRVisualization|TrasladarRamaPressed))
          (:ERotationTask
            ;[0.155 0.155 0.155] Tarea Rotar Rama, se selecciona un nodo que es el que hace la referencia el inidio de la rama a rotar respecto al padre del nodo seleccionadom, lo malo es que provocara coloración, lo cual no esta bien creo
            (if (Variables|Default|GetbHitNodo)
              (Variables|Default|SetbNodoGuia true)
              (bind _output_get_2 (Variables|Default|SetNodoGuia (Variables|Default|GetHitNodo)))
              (Class|VRVisualization|SeleccionarRama _output_get_2)))))
      (:ENoMode
        ;[1 1 1] Visualizacion
        (bind _returnvalue_6 (Class|VRVisualization|GetVisualizationTask))
        (switch Utilities|FlowControl|Switch|SwitchonEVRVisualizationTask _returnvalue_6
          (:ETraslationTask
            (Class|VRVisualization|TrasladarVisualizacionPressed))
          (:ERotationTask
            (Class|VRVisualization|RotarVisualizacionPressed))))))
  (:Released
    (bind _returnvalue_7 (Class|VRVisualization|GetVisualizationMode))
    (switch Utilities|FlowControl|Switch|SwitchonEVRVisualizationMode _returnvalue_7
      (:EAll
        ;[1 1 1] Todo
        (bind _returnvalue_8 (Class|VRVisualization|GetVisualizationTask))
        (switch Utilities|FlowControl|Switch|SwitchonEVRVisualizationTask _returnvalue_8
          (:ETraslationTask
            (Class|VRVisualization|TrasladarTodoReleased))))
      (:ENode
        ;[1 1 1] Nodo
        (bind _returnvalue_9 (Class|VRVisualization|GetVisualizationTask))
        (switch Utilities|FlowControl|Switch|SwitchonEVRVisualizationTask _returnvalue_9
          (:ETraslationTask
            (Class|VRVisualization|TrasladarNodoReleased))
          (:EVisualizationTask
            (Class|VRVisualization|VisualizarNodoReleased))))
      (:EBranch
        ;[1 1 1] Rama
        (bind _returnvalue_10 (Class|VRVisualization|GetVisualizationTask))
        (switch Utilities|FlowControl|Switch|SwitchonEVRVisualizationTask _returnvalue_10
          (:ETraslationTask
            (Class|VRVisualization|TrasladarRamaReleased))
          (:ERotationTask
            (Class|VRVisualization|RotarRamaReleased))))
      (:ENoMode
        ;[1 1 1] Visualizacion
        (bind _returnvalue_11 (Class|VRVisualization|GetVisualizationTask))
        (switch Utilities|FlowControl|Switch|SwitchonEVRVisualizationTask _returnvalue_11
          (:ETraslationTask
            (Class|VRVisualization|TrasladarVisualizacionReleased))
          (:ERotationTask
            (Class|VRVisualization|RotarVisualizacionReleased)))))))

(event Input|ActionEvents|InputActionTaskSelection
  (params (Key :type Key%20Structure))
  ;[0.155 0.155 0.155] Visualization Tasks
  (:Pressed
    (Class|VRVisualization|SetVisualizationTask "ENoTask")
    (Development|PrintText "Seleccionar" true true "(R=0.000000,G=0.475000,B=0.018212,A=1.000000)" 5.0)))

(event Input|ActionEvents|InputActionTaskTraslation
  (params (Key :type Key%20Structure))
  ;[0.155 0.155 0.155] Visualization Tasks
  (:Pressed
    (Class|VRVisualization|SetVisualizationTask "ETraslationTask")
    (Development|PrintText "Trasladar" true true "(R=0.000000,G=0.475000,B=0.018212,A=1.000000)" 5.0)))

(event Input|ActionEvents|InputActionTaskRotation
  (params (Key :type Key%20Structure))
  ;[0.155 0.155 0.155] Visualization Tasks
  (:Pressed
    (Class|VRVisualization|SetVisualizationTask "ERotationTask")
    (Development|PrintText "Rotar" true true "(R=0.000000,G=0.475000,B=0.018212,A=1.000000)" 5.0)))

(event Input|ActionEvents|InputActionTaskVisualization
  (params (Key :type Key%20Structure))
  ;[0.155 0.155 0.155] Visualization Tasks
  (:Pressed
    (Class|VRVisualization|SetVisualizationTask "EVisualizationTask")
    (Development|PrintText "Visaulizar" true true "(R=0.000000,G=0.475000,B=0.018212,A=1.000000)" 5.0)))

(event Input|ActionEvents|InputActionTaskNone
  (params (Key :type Key%20Structure))
  ;[0.155 0.155 0.155] Visualization Tasks
  (:Pressed
    (Class|VRVisualization|SetVisualizationTask "ENoTask")
    (Development|PrintText "Ninguno" true true "(R=0.000000,G=0.475000,B=0.018212,A=1.000000)" 5.0)))

(fn ConstructionScript)