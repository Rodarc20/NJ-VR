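; PolyPlane VR visualization Blueprint that lets the player scale, move, rotate and inspect a node-and-edge layout with motion controllers.
; Holding both grips captures the controller distance and applies a temporary scale each Tick, committed on release.
; Tick and Select input dispatch by visualization mode (node, branch, all, none) and task to helper functions for laser picking, translation and rotation.
; Selecting a node in Visualizar task fills and shows its content widget.
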(event EventBeginPlay)

(event Collision|EventActorBeginOverlap
  (params (OtherActor :type Actor%20Object%20Reference)))

(event EventTick
  (params (DeltaSeconds :type Float%20%28single-precision%29))
  ;[1 1 1] esto deberia estar dentro de una sola funcion
  (if (Variables|Default|GetbCalcularEscala)
    (Class|VRVisualization|CalcularEscalaTemporal)
    (Class|VRVisualization|AplicarEscala (Variables|Default|GetEscalaTemp)))
  (bind _returnvalue (Class|VRVisualization|GetVisualizationMode))
  ;[1 1 1] seleccionar el modo, sin area tengo 4, no selecciona es la visualizacion completa
  (switch Utilities|FlowControl|Switch|SwitchonEVRVisualizationMode _returnvalue
    (:ENode
      ;[1 1 1] Nodo
      (bind _returnvalue_2 (Class|VRVisualization|GetVisualizationTask))
      ;;[1 1 1] la tarea seleccionar esta impicata en todos los otrso mdos, el ninguno deberia tener su propia funcion apra manipular laser apuntando e menu, no como esta ahora
      (switch Utilities|FlowControl|Switch|SwitchonEVRVisualizationTask _returnvalue_2
        (:ETraslationTask
          ;[1 1 1] esto deberia estar dentro de una sola funcion???
          (if (Variables|Default|GetbNodoGuia)
            (Class|VRVisualization|TraslacionConNodoGuia)
            (else
              (Class|VRVisualization|BuscandoNodoConLaser :!label _label))))
        (:EVisualizationTask
          (Class|VRVisualization|VisualizarNodo))
        (:ENoTask
          (goto _label))))
    (:EBranch
      ;[1 1 1] Rama
      (bind _returnvalue_3 (Class|VRVisualization|GetVisualizationTask))
      (switch Utilities|FlowControl|Switch|SwitchonEVRVisualizationTask _returnvalue_3
        (:ETraslationTask
          (if (Variables|Default|GetbNodoGuia)
            (Class|VRVisualization|TraslacionConNodoGuia)
            (else
              (Class|VRVisualization|BuscandoNodoConLaser :!label _label_2))))
        (:ERotationTask
          (if (not (Variables|Default|GetbNodoGuia))
            (goto _label_2)))))
    (:ENoMode
      ;[1 1 1] Visualización, la tarea visualizacion solo deberia marcar dentro del menu
      (bind _returnvalue_4 (Class|VRVisualization|GetVisualizationTask))
      (switch Utilities|FlowControl|Switch|SwitchonEVRVisualizationTask _returnvalue_4
        (:ETraslationTask
          (if (Variables|Default|GetbNodoGuia)
            (Class|VRVisualization|TraslacionVisualizacion)
            (else
              (Class|VRVisualization|BuscandoNodoConLaser :!label _label_3))))
        (:ERotationTask
          (if (Variables|Default|GetRotar)
            (Class|VRVisualization|RotarVisualizacion)
            (goto _label_3)
            (else
              (goto _label_3))))
        (:EVisualizationTask
          (goto _label_3))
        (:ENoTask
          (goto _label_3))))))

(event Input|ActionEvents|InputActionSostenerDerecha
  (params (Key :type Key%20Structure))
  ;[0.055 0.055 0.055] Escala
  (:Pressed
    (Variables|Default|SetbGripDerecho true)
    (if (Variables|Default|GetbGripIzquierdo)
      (Variables|Default|SetbCalcularEscala true)
      (Variables|Default|SetDistanciaInicialControles (Math|Vector|VectorLength (- (Transformation|GetWorldLocation (Variables|Default|GetRightController)) (Transformation|GetWorldLocation (Variables|Default|GetLeftController)))))))
  (:Released
    (Variables|Default|SetbGripDerecho false)
    (Variables|Default|SetbCalcularEscala false)
    (bind _output_get (Variables|Default|SetEscala (Variables|Default|GetEscalaTemp)))
    (Class|VRVisualization|AplicarEscala _output_get)))

(event Input|ActionEvents|InputActionSostenerIzquierda
  (params (Key :type Key%20Structure))
  ;[0.055 0.055 0.055] Escala
  (:Pressed
    (Variables|Default|SetbGripIzquierdo true)
    (if (Variables|Default|GetbGripDerecho)
      (Variables|Default|SetbCalcularEscala true)
      (Variables|Default|SetDistanciaInicialControles (Math|Vector|VectorLength (- (Transformation|GetWorldLocation (Variables|Default|GetRightController)) (Transformation|GetWorldLocation (Variables|Default|GetLeftController)))))))
  (:Released
    (Variables|Default|SetbGripIzquierdo false)
    (Variables|Default|SetbCalcularEscala false)
    (bind _output_get (Variables|Default|SetEscala (Variables|Default|GetEscalaTemp)))
    (Class|VRVisualization|AplicarEscala _output_get)))

(event Input|ActionEvents|InputActionSelect
  (params (Key :type Key%20Structure))
  (bind _hitnodo (Variables|Default|GetHitNodo))
  (:Pressed
    (bind _returnvalue (Class|VRVisualization|GetVisualizationMode))
    (switch Utilities|FlowControl|Switch|SwitchonEVRVisualizationMode _returnvalue
      (:EAll
        ;[1 1 1] Todo
        (bind _returnvalue_2 (Class|VRVisualization|GetVisualizationTask))
        (switch Utilities|FlowControl|Switch|SwitchonEVRVisualizationTask _returnvalue_2
          (:ETraslationTask
            (Class|VRVisualization|TrasladarTodoPressed))))
      (:ENode
        ;[1 1 1] Nodo
        (bind _returnvalue_3 (Class|VRVisualization|GetVisualizationTask))
        (switch Utilities|FlowControl|Switch|SwitchonEVRVisualizationTask _returnvalue_3
          (:ETraslationTask
            (Class|VRVisualization|TrasladarNodoPressed))
          (:EVisualizationTask
            (Class|VRVisualization|VisualizarNodoPressed)
            (if (Variables|Default|GetbHitNodo)
              ;[1 1 1] VisualizarNodoPressed
              (bind _ascontenido_nodo (Utilities|Casting|CastToContenidoNodo (UserInterface|GetUserWidgetObject (Variables|/Script/NJVR.Nodo|GetContenido _hitnodo))))
              (bind _output_get (Variables|/Game/Visualization/Blueprints/Menu/ContenidoNodo.ContenidoNodo_C|SetNodo _ascontenido_nodo _hitnodo))
              (bind _returnvalue_4 (Class|VRVisualization|ObtenerContenidoNodo _output_get))
              (Default|CambiarTexto _ascontenido_nodo (Utilities|Text|ToText(String) _returnvalue_4))
              (Class|Nodo|MostrarContenido _hitnodo)))))
      (:EBranch
        ;[1 1 1] Rama
        (bind _returnvalue_5 (Class|VRVisualization|GetVisualizationTask))
        (switch Utilities|FlowControl|Switch|SwitchonEVRVisualizationTask _returnvalue_5
          (:ETraslationTask
            (Class|VRVisualization|TrasladarRamaPressed))))
      (:ENoMode
        ;[1 1 1] Visualizacion
        (bind _returnvalue_6 (Class|VRVisualization|GetVisualizationTask))
        (switch Utilities|FlowControl|Switch|SwitchonEVRVisualizationTask _returnvalue_6
          (:ETraslationTask
            (Class|VRVisualization|TrasladarVisualizacionPressed))
          (:ERotationTask
            (Class|VRVisualization|RotarVisualizacionPressed))))))
  (:Released
    (bind _returnvalue_7 (Class|VRVisualization|GetVisualizationMode))
    (switch Utilities|FlowControl|Switch|SwitchonEVRVisualizationMode _returnvalue_7
      (:ENode
        ;[1 1 1] Nodo
        (bind _returnvalue_8 (Class|VRVisualization|GetVisualizationTask))
        (switch Utilities|FlowControl|Switch|SwitchonEVRVisualizationTask _returnvalue_8
          (:ETraslationTask
            (Class|VRVisualization|TrasladarNodoReleased))
          (:EVisualizationTask
            (Class|VRVisualization|VisualizarNodoReleased))))
      (:EBranch
        ;[1 1 1] Rama
        (bind _returnvalue_9 (Class|VRVisualization|GetVisualizationTask))
        (switch Utilities|FlowControl|Switch|SwitchonEVRVisualizationTask _returnvalue_9
          (:ETraslationTask
            (Class|VRVisualization|TrasladarRamaReleased))))
      (:ENoMode
        ;[1 1 1] Visualizacion
        (bind _returnvalue_10 (Class|VRVisualization|GetVisualizationTask))
        (switch Utilities|FlowControl|Switch|SwitchonEVRVisualizationTask _returnvalue_10
          (:ETraslationTask
            (Class|VRVisualization|TrasladarVisualizacionReleased))
          (:ERotationTask
            (Class|VRVisualization|RotarVisualizacionReleased)))))))

(fn ConstructionScript)