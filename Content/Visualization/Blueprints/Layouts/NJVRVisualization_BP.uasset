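; VR controller for a node-and-edge visualization with branches, letting the player select, move, rotate, scale and inspect it.
; Input actions set a mode (all, node, branch, area, none) and task; Select applies that pair.
; Tick draws the right-controller laser, tracing nodes to pick or a board to drag against; mode none moves the whole actor.
; Gripping both controllers rescales by hand distance; visualizing a node shows its content in the pawn's Document widget.
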(event EventBeginPlay
  (bind _asvrpawn_2vrv_bp (Utilities|Casting|CastToVRPawn2VRV_BP (Game|Player|GetPlayerPawn 0)))
  (Variables|Default|SetRightController (Variables|/Game/ControllerSetup/VRPawn2VRV_BP.VRPawn2VRV_BP_C|GetMotionControllerRight _asvrpawn_2vrv_bp))
  (Variables|Default|SetLeftController (Variables|/Game/ControllerSetup/VRPawn2VRV_BP.VRPawn2VRV_BP_C|GetMotionControllerLeft _asvrpawn_2vrv_bp))
  (Variables|/Game/ControllerSetup/VRPawn2VRV_BP.VRPawn2VRV_BP_C|SetVisualization _asvrpawn_2vrv_bp self)
  (Variables|Default|SetInteraction (Variables|/Game/ControllerSetup/VRPawn2VRV_BP.VRPawn2VRV_BP_C|GetInteraction _asvrpawn_2vrv_bp))
  (Variables|Default|SetDocument (Variables|/Game/ControllerSetup/VRPawn2VRV_BP.VRPawn2VRV_BP_C|GetDocument _asvrpawn_2vrv_bp)))

(event EventTick
  (params (DeltaSeconds :type Float%20%28single-precision%29))
  (bind _distancialaser (Variables|Default|GetDistanciaLaser))
  (bind _rightcontroller (Variables|Default|GetRightController))
  (bind _distanciainicialcontroles (Variables|Default|GetDistanciaInicialControles))
  (bind _rightcontroller_2 (Variables|Default|GetRightController))
  (bind _rightcontroller_3 (Variables|Default|GetRightController))
  (bind _mostrarlabel (Variables|Default|GetMostrarLabel))
  (bind _rightcontroller_4 (Variables|Default|GetRightController))
  (bind _returnvalue (Transformation|GetWorldLocation _rightcontroller))
  (bind _returnvalue_2 (Math|Vector|GetForwardVector _rightcontroller_4))
  (bind _returnvalue_3 (Math|Vector|GetForwardVector _rightcontroller))
  (bind _returnvalue_4 (Transformation|GetWorldLocation _rightcontroller_4))
  (bind _returnvalue_5 (Transformation|GetWorldLocation _rightcontroller_2))
  (bind _returnvalue_6 (Math|Vector|GetForwardVector _rightcontroller_2))
  (bind _returnvalue_7 (Transformation|GetWorldLocation _rightcontroller_3))
  (bind _returnvalue_8 (Math|Vector|GetForwardVector _rightcontroller_3))
  (bind _returnvalue_9 (* _returnvalue_3 1e+03))
  (bind _returnvalue_10 (* _returnvalue_2 _distancialaser))
  (bind _returnvalue_11 (* _returnvalue_8 1e+03))
  (bind _returnvalue_12 (* _returnvalue_6 1e+03))
  (bind _returnvalue_13 (+ _returnvalue _returnvalue_9))
  (bind _returnvalue_14 (+ _returnvalue_4 _returnvalue_10))
  (bind _returnvalue_15 (+ _returnvalue_5 _returnvalue_12))
  (bind _returnvalue_16 (+ _returnvalue_7 _returnvalue_11))
  (if (Variables|Default|GetbCalcularEscala)
    (bind _output_get (Variables|Default|SetEscalaTemp (+ (Variables|Default|GetEscala) (/ (- (Math|Vector|VectorLength (- (Transformation|GetWorldLocation (Variables|Default|GetRightController)) (Transformation|GetWorldLocation (Variables|Default|GetLeftController)))) _distanciainicialcontroles) _distanciainicialcontroles))))
    (Class|VRVisualization|AplicarEscala _output_get)
    (bind _returnvalue_17 (Class|VRVisualization|GetVisualizationMode))
    ;[1 1 1] seleccionar el modo, sin area tengo 4, no selecciona es la visualizacion completa
    (switch Utilities|FlowControl|Switch|SwitchonEVRVisualizationMode _returnvalue_17
      (:EAll
        ;[1 1 1] Todo
        (bind _returnvalue_18 (Class|VRVisualization|GetVisualizationTask))
        (switch Utilities|FlowControl|Switch|SwitchonEVRVisualizationTask _returnvalue_18
          (:ETraslationTask
            (if (Variables|Default|GetbNodoGuia)
              ;[0.155 0.155 0.155] Buscar un punto en los limites de la visualizacion don de trasladar los nodos, este puedesta cosa puede ser reemplazada por calculos
              (bind (_outhit _returnvalue_19) (Collision|LineTraceForObjects _returnvalue_5 _returnvalue_15 (Utilities|Array|MakeArray "ObjectTypeQuery9") false 0 "None" false :!label _label))
              (bind _output_get_2 (Variables|Default|SetbHitBoard _returnvalue_19))
              (Variables|Default|SetHitActor (.HitActor (Collision|BreakHitResult _outhit)))
              (if _output_get_2
                (Rendering|Debug|DrawDebugLine _returnvalue_5 (.ImpactPoint (Collision|BreakHitResult _outhit)) "(R=0.000000,G=0.475000,B=0.018212,A=1.000000)" 0.0 0.5)
                (Class|VRVisualization|AplicarTraslacion (- (.ImpactPoint (Collision|BreakHitResult _outhit)) (Transformation|GetActorLocation (Variables|Default|GetNodoGuia))))
                (else
                  (Rendering|Debug|DrawDebugLine _returnvalue_5 _returnvalue_15 "(R=0.905000,G=0.000000,B=0.000000,A=1.000000)" 0.0 0.5)))
              (else
                ;[0.155 0.155 0.155] Para dibujar el laser que busca un nodo para seleccionar, esta accion siempre se hace, y se termina cuando presiono el trigger
                (bind (_outhit_2 _returnvalue_20) (Collision|LineTraceForObjects (+ _returnvalue_7 (* _returnvalue_8 2e+01)) _returnvalue_16 (Utilities|Array|MakeArray "ObjectTypeQuery8" "ObjectTypeQuery2") false 0 "None" :!label _label_2))
                (bind _asnodo (Utilities|Casting|CastToNodo (.HitActor (Collision|BreakHitResult _outhit_2)))
                  (:then
                    (bind _output_get_3 (Variables|Default|SetHitNodo _asnodo))
                    (if _mostrarlabel
                      (Class|Nodo|MostrarNombre _output_get_3))
                    (Variables|Default|SetbHitNodo true))
                  (:CastFailed
                    (if _mostrarlabel
                      (if (Utilities|IsValid (Variables|Default|GetHitNodo))
                        (Class|Nodo|OcultarNombre (Variables|Default|GetHitNodo))
                        (Variables|Default|SetHitNodo 0)))
                    (Variables|Default|SetbHitNodo false)))
                (Variables|Default|SetHitActor (.HitActor (Collision|BreakHitResult _outhit_2)))
                (bind _output_get_4 (Variables|Default|SetImpactPoint (.ImpactPoint (Collision|BreakHitResult _outhit_2))))
                (Rendering|Debug|DrawDebugLine _returnvalue_7 (Math|Vector|SelectVector _output_get_4 _returnvalue_16 _returnvalue_20) "(R=0.004780,G=0.000000,B=0.905000,A=1.000000)" 0.0 0.5)
                (if _returnvalue_20
                  (Rendering|Debug|DrawDebugCircle _output_get_4 1.5 5 "(R=0.000000,G=0.000000,B=0.000000,A=1.000000)" 0.0 2.0 "0.000000,1.000000,0.000000" "0.000000,0.000000,1.000000")))))
          (:ENoTask
            (goto _label_2))))
      (:ENode
        ;[1 1 1] Nodo
        (bind _returnvalue_21 (Class|VRVisualization|GetVisualizationTask))
        ;;[1 1 1] la tarea seleccionar esta impicata en todos los otrso mdos
        (switch Utilities|FlowControl|Switch|SwitchonEVRVisualizationTask _returnvalue_21
          (:ETraslationTask
            (if (Variables|Default|GetbNodoGuia)
              (goto _label)
              (else
                (goto _label_2))))
          (:EVisualizationTask
            (goto _label_2))
          (:ENoTask
            (goto _label_2))))
      (:EBranch
        ;[1 1 1] Rama
        (bind _returnvalue_22 (Class|VRVisualization|GetVisualizationTask))
        (switch Utilities|FlowControl|Switch|SwitchonEVRVisualizationTask _returnvalue_22
          (:ETraslationTask
            (if (Variables|Default|GetbNodoGuia)
              (goto _label)
              (else
                (goto _label_2))))
          (:ERotationTask
            (if (Variables|Default|GetbNodoGuia)
              ;[0.155 0.155 0.155] Tarea Rotar Rama
              (bind (_outhit_3 _returnvalue_23) (Collision|LineTraceForObjects _returnvalue _returnvalue_13 (Utilities|Array|MakeArray "ObjectTypeQuery9") false 0 "None" false))
              (bind _output_get_5 (Variables|Default|SetbHitBoard _returnvalue_23))
              (Variables|Default|SetHitActor (.HitActor (Collision|BreakHitResult _outhit_3)))
              (if _output_get_5
                (Rendering|Debug|DrawDebugLine _returnvalue (.ImpactPoint (Collision|BreakHitResult _outhit_3)) "(R=0.000000,G=0.475000,B=0.018212,A=1.000000)" 0.0 0.5)
                (Class|VRVisualization|AplicarRotacionRelativaANodo (Variables|Default|GetNodoGuia) (.ImpactPoint (Collision|BreakHitResult _outhit_3)))
                (else
                  (Rendering|Debug|DrawDebugLine _returnvalue _returnvalue_13 "(R=0.905000,G=0.000000,B=0.000000,A=1.000000)" 0.0 0.5)))
              (else
                (goto _label_2))))
          (:ENoTask
            (goto _label_2))))
      (:ENoMode
        ;[1 1 1] Visualización, la tarea visualizacion solo deberia marcar dentro del menu
        (bind _returnvalue_24 (Class|VRVisualization|GetVisualizationTask))
        (switch Utilities|FlowControl|Switch|SwitchonEVRVisualizationTask _returnvalue_24
          (:ETraslationTask
            (if (Variables|Default|GetbNodoGuia)
              (Transformation|SetActorLocation (+ _returnvalue_14 (Variables|Default|GetOffsetToPointLaser)) false false)
              (Rendering|Debug|DrawDebugLine _returnvalue_4 _returnvalue_14 "(R=0.222584,G=0.000000,B=0.300000,A=1.000000)" 0.0 0.5)
              (else
                (goto _label_2))))
          (:ERotationTask
            ;[0.155 0.155 0.155] Tarea Rotar
            (if (Variables|Default|GetRotar)
              (Transformation|SetActorRotation (Math|Rotator|CombineRotators (Variables|Default|GetInitialRotation) (Math|Rotator|Delta(Rotator) (Transformation|GetWorldRotation (Variables|Default|GetRightController)) (Variables|Default|GetInitialRotationController))))
              (goto _label_2)
              (else
                (goto _label_2))))
          (:EVisualizationTask
            (goto _label_2))
          (:ENoTask
            (goto _label_2)))))))

(event Input|ActionEvents|InputActionModeAll
  (params (Key :type Key%20Structure :default "AnyKey"))
  ;[0.155 0.155 0.155] Visualizations Modes
  (:Pressed
    (Variables|Default|SetCurrentVisualizationMode "EAll")
    (Development|PrintText "Todo" true true "(R=0.000000,G=0.056297,B=1.000000,A=1.000000)" 5.0)))

(event Input|ActionEvents|InputActionModeIndividual
  (params (Key :type Key%20Structure :default "AnyKey"))
  ;[0.155 0.155 0.155] Visualizations Modes
  (:Pressed
    ;;[1 1 1] COmo la variable es de esta clase, puedo modificarla directamente
    (Variables|Default|SetCurrentVisualizationMode "ENode")
    (Development|PrintText "Nodo por nodo" true true "(R=0.000000,G=0.056297,B=1.000000,A=1.000000)" 5.0)))

(event Input|ActionEvents|InputActionModeBranch
  (params (Key :type Key%20Structure :default "AnyKey"))
  ;[0.155 0.155 0.155] Visualizations Modes
  (:Pressed
    (Variables|Default|SetCurrentVisualizationMode "EBranch")
    (Development|PrintText "Rama" true true "(R=0.000000,G=0.056297,B=1.000000,A=1.000000)" 5.0)))

(event Input|ActionEvents|InputActionModeArea
  (params (Key :type Key%20Structure :default "AnyKey"))
  ;[0.155 0.155 0.155] Visualizations Modes
  (:Pressed
    ;;[1 1 1] pero lo correcto seria usar el setter
    (Class|VRVisualization|SetVisualizationMode "EArea")
    (Development|PrintText "Area" true true "(R=0.000000,G=0.056297,B=1.000000,A=1.000000)" 5.0)))

(event Input|ActionEvents|InputActionModeNone
  (params (Key :type Key%20Structure :default "AnyKey"))
  ;[0.155 0.155 0.155] Visualizations Modes
  (:Pressed
    (Class|VRVisualization|SetVisualizationMode "ENoMode")
    (Development|PrintText "Ninguno" true true "(R=0.000000,G=0.056297,B=1.000000,A=1.000000)" 5.0)
    ;;[1 1 1] EStos al no requerir dar click en algun nodo, automaticamente edeben ser ejecutados al entrar en ese modo
    (Class|VRVisualization|DeseleccionarTodo)))

(event Input|ActionEvents|InputActionSostenerDerecha
  (params (Key :type Key%20Structure :default "AnyKey"))
  ;[0.055 0.055 0.055] Escala
  (:Pressed
    (Variables|Default|SetbGripDerecho true)
    (if (Variables|Default|GetbGripIzquierdo)
      (Variables|Default|SetbCalcularEscala true)
      (Variables|Default|SetDistanciaInicialControles (Math|Vector|VectorLength (- (Transformation|GetWorldLocation (Variables|Default|GetRightController)) (Transformation|GetWorldLocation (Variables|Default|GetLeftController)))))
      (for _array_element (Variables|Default|GetNodos)
        (Utilities|Array|Add (Variables|Default|GetPosicionesNodosInicialEscala) (.Location (Math|Transform|BreakTransform (Transformation|GetActorTransform _array_element)))))))
  (:Released
    (Variables|Default|SetbGripDerecho false)
    (Variables|Default|SetbCalcularEscala false)
    (bind _output_get (Variables|Default|SetEscala (Variables|Default|GetEscalaTemp)))
    (Class|VRVisualization|AplicarEscala _output_get)))

(event Input|ActionEvents|InputActionSostenerIzquierda
  (params (Key :type Key%20Structure :default "AnyKey"))
  ;[0.055 0.055 0.055] Escala
  (:Pressed
    (Variables|Default|SetbGripIzquierdo true)
    (if (Variables|Default|GetbGripDerecho)
      (Variables|Default|SetbCalcularEscala true)
      (Variables|Default|SetDistanciaInicialControles (Math|Vector|VectorLength (- (Transformation|GetWorldLocation (Variables|Default|GetRightController)) (Transformation|GetWorldLocation (Variables|Default|GetLeftController)))))
      (for _array_element (Variables|Default|GetNodos)
        (Utilities|Array|Add (Variables|Default|GetPosicionesNodosInicialEscala) (.Location (Math|Transform|BreakTransform (Transformation|GetActorTransform _array_element)))))))
  (:Released
    (Variables|Default|SetbGripIzquierdo false)
    (Variables|Default|SetbCalcularEscala false)
    (bind _output_get (Variables|Default|SetEscala (Variables|Default|GetEscalaTemp)))
    (Class|VRVisualization|AplicarEscala _output_get)))

(event Input|ActionEvents|InputActionSelect
  (params (Key :type Key%20Structure :default "AnyKey"))
  (bind _document (Variables|Default|GetDocument))
  (bind _hitnodo (Variables|Default|GetHitNodo))
  (bind _bhitnodo (Variables|Default|GetbHitNodo))
  (bind _impactpoint (Variables|Default|GetImpactPoint))
  (:Pressed
    (bind _returnvalue (Class|VRVisualization|GetVisualizationMode))
    (switch Utilities|FlowControl|Switch|SwitchonEVRVisualizationMode _returnvalue
      (:EAll
        ;[1 1 1] Todo
        (bind _returnvalue_2 (Class|VRVisualization|GetVisualizationTask))
        (switch Utilities|FlowControl|Switch|SwitchonEVRVisualizationTask _returnvalue_2
          (:ETraslationTask
            (Class|VRVisualization|SeleccionarTodo)
            (if _bhitnodo
              (Variables|Default|SetNodoGuia _hitnodo)
              (Variables|Default|SetbNodoGuia true)))))
      (:ENode
        ;[1 1 1] Nodo
        (bind _returnvalue_3 (Class|VRVisualization|GetVisualizationTask))
        (switch Utilities|FlowControl|Switch|SwitchonEVRVisualizationTask _returnvalue_3
          (:ETraslationTask
            (if _bhitnodo
              ;[1 1 1] seleccion
              (Class|VRVisualization|SeleccionarNodo _hitnodo)
              ;[1 1 1] preparacion para traslado
              (Variables|Default|SetNodoGuia _hitnodo)
              (Variables|Default|SetbNodoGuia true)))
          (:EVisualizationTask
            (if _bhitnodo
              ;[1 1 1] eso es solo por ahora, cuando llegue a abrir el documento cambiara
              (Class|VRVisualization|SeleccionarNodo _hitnodo)
              (Class|Nodo|MostrarNombre _hitnodo)
              (bind _ascontrol_menu_2vr (Utilities|Casting|CastToControlMenu2VR (UserInterface|GetUserWidgetObject _document)))
              (bind _returnvalue_4 (Class|VRVisualization|ObtenerContenidoNodo _hitnodo))
              ;[0.055 0.055 0.055] Del menu para le contenido
              (Default|CambiarTexto _ascontrol_menu_2vr (Utilities|Text|ToText(String) _returnvalue_4))
              (Collision|SetCollisionObjectType _document "ECC_WorldDynamic")
              (Rendering|SetVisibility _document true true)))))
      (:EBranch
        ;[1 1 1] Rama
        (bind _returnvalue_5 (Class|VRVisualization|GetVisualizationTask))
        (switch Utilities|FlowControl|Switch|SwitchonEVRVisualizationTask _returnvalue_5
          (:ETraslationTask
            (if _bhitnodo
              (Class|VRVisualization|SeleccionarRama _hitnodo)
              ;[1 1 1] preparacion para traslado
              (Variables|Default|SetNodoGuia _hitnodo)
              (Variables|Default|SetbNodoGuia true)))
          (:ERotationTask
            ;[0.155 0.155 0.155] Tarea Rotar Rama, se selecciona un nodo que es el que hace la referencia el inidio de la rama a rotar respecto al padre del nodo seleccionadom, lo malo es que provocara coloración, lo cual no esta bien creo
            (if _bhitnodo
              (Variables|Default|SetbNodoGuia true)
              (bind _output_get (Variables|Default|SetNodoGuia _hitnodo))
              (Class|VRVisualization|SeleccionarRama _output_get)))))
      (:ENoMode
        ;[1 1 1] Visualizacion
        (bind _returnvalue_6 (Class|VRVisualization|GetVisualizationTask))
        (switch Utilities|FlowControl|Switch|SwitchonEVRVisualizationTask _returnvalue_6
          (:ETraslationTask
            (Variables|Default|SetDistanciaLaser (Math|Vector|VectorLength (- _impactpoint (Transformation|GetWorldLocation (Variables|Default|GetRightController)))))
            (Variables|Default|SetOffsetToPointLaser (- (Transformation|GetActorLocation) _impactpoint))
            ;[0 0.01 0.000383] Usare el bool de nodo guia, pero no deberia usarlo
            (Variables|Default|SetbNodoGuia true))
          (:ERotationTask
            ;[0.155 0.155 0.155] Tarea Rotar
            (Variables|Default|SetInitialRotationController (Transformation|GetWorldRotation (Variables|Default|GetRightController)))
            (Variables|Default|SetInitialRotation (Transformation|GetActorRotation))
            (Variables|Default|SetRotar true))))))
  (:Released
    (bind _returnvalue_7 (Class|VRVisualization|GetVisualizationMode))
    (switch Utilities|FlowControl|Switch|SwitchonEVRVisualizationMode _returnvalue_7
      (:EAll
        ;[1 1 1] Todo
        (bind _returnvalue_8 (Class|VRVisualization|GetVisualizationTask))
        (switch Utilities|FlowControl|Switch|SwitchonEVRVisualizationTask _returnvalue_8
          (:ETraslationTask
            (Class|VRVisualization|DeseleccionarTodo)
            (Variables|Default|SetbNodoGuia false))))
      (:ENode
        ;[1 1 1] Nodo
        (bind _returnvalue_9 (Class|VRVisualization|GetVisualizationTask))
        (switch Utilities|FlowControl|Switch|SwitchonEVRVisualizationTask _returnvalue_9
          (:ETraslationTask
            ;[0.155 0.155 0.155] Tarea Trasladar
            (Class|VRVisualization|DeseleccionarTodo)
            (Variables|Default|SetbNodoGuia false)
            (for _array_element (Variables|Default|GetAristas)
              (Class|Arista|ActualizarCollision _array_element)))
          (:EVisualizationTask
            (for _array_element_2 (Variables|Default|GetNodosSeleccionados)
              (Class|Nodo|OcultarNombre _array_element_2))
            (Class|VRVisualization|DeseleccionarTodo))))
      (:EBranch
        ;[1 1 1] Rama
        (bind _returnvalue_10 (Class|VRVisualization|GetVisualizationTask))
        (switch Utilities|FlowControl|Switch|SwitchonEVRVisualizationTask _returnvalue_10
          (:ETraslationTask
            (Class|VRVisualization|DeseleccionarRama (Variables|Default|GetNodoGuia))
            (Variables|Default|SetbNodoGuia false)
            (for _array_element_3 (Variables|Default|GetAristas)
              (Class|Arista|ActualizarCollision _array_element_3)))
          (:ERotationTask
            (Variables|Default|SetbNodoGuia false)
            (for _array_element_4 (Variables|Default|GetAristas)
              (Class|Arista|ActualizarCollision _array_element_4))
            (Class|VRVisualization|DeseleccionarTodo))))
      (:ENoMode
        ;[1 1 1] Visualizacion
        (bind _returnvalue_11 (Class|VRVisualization|GetVisualizationTask))
        (switch Utilities|FlowControl|Switch|SwitchonEVRVisualizationTask _returnvalue_11
          (:ETraslationTask
            (Variables|Default|SetbNodoGuia false)
            (for _array_element_5 (Variables|Default|GetAristas)
              (Class|Arista|ActualizarCollision _array_element_5)))
          (:ERotationTask
            ;[0.155 0.155 0.155] Tarea Rotar
            (Variables|Default|SetRotar false)))))))

(event Input|ActionEvents|InputActionTaskSelection
  (params (Key :type Key%20Structure :default "AnyKey"))
  ;[0.155 0.155 0.155] Visualization Tasks
  (:Pressed
    (Class|VRVisualization|SetVisualizationTask "ENoTask")
    (Development|PrintText "Seleccionar" true true "(R=0.000000,G=0.475000,B=0.018212,A=1.000000)" 5.0)))

(event Input|ActionEvents|InputActionTaskTraslation
  (params (Key :type Key%20Structure :default "AnyKey"))
  ;[0.155 0.155 0.155] Visualization Tasks
  (:Pressed
    (Class|VRVisualization|SetVisualizationTask "ETraslationTask")
    (Development|PrintText "Trasladar" true true "(R=0.000000,G=0.475000,B=0.018212,A=1.000000)" 5.0)))

(event Input|ActionEvents|InputActionTaskRotation
  (params (Key :type Key%20Structure :default "AnyKey"))
  ;[0.155 0.155 0.155] Visualization Tasks
  (:Pressed
    (Class|VRVisualization|SetVisualizationTask "ERotationTask")
    (Development|PrintText "Rotar" true true "(R=0.000000,G=0.475000,B=0.018212,A=1.000000)" 5.0)))

(event Input|ActionEvents|InputActionTaskVisualization
  (params (Key :type Key%20Structure :default "AnyKey"))
  ;[0.155 0.155 0.155] Visualization Tasks
  (:Pressed
    (Class|VRVisualization|SetVisualizationTask "EVisualizationTask")
    (Development|PrintText "Visaulizar" true true "(R=0.000000,G=0.475000,B=0.018212,A=1.000000)" 5.0)))

(event Input|ActionEvents|InputActionTaskNone
  (params (Key :type Key%20Structure :default "AnyKey"))
  ;[0.155 0.155 0.155] Visualization Tasks
  (:Pressed
    (Class|VRVisualization|SetVisualizationTask "ENoTask")
    (Development|PrintText "Ninguno" true true "(R=0.000000,G=0.475000,B=0.018212,A=1.000000)" 5.0)))

(fn ConstructionScript)