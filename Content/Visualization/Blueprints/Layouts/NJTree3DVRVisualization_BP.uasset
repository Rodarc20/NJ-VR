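; Visualization Blueprint for a 3D VR NJ tree layout that can swap its node and edge actors for mesh instances.
; Pressing Right Ctrl hides each node mesh and copies its transform into NodosH if valid, enlarged 1.5x, or NodosVH otherwise.
; Edges cast to AristaCilindro are likewise hidden and copied into AristasH, with debug prints along the way.
; Tick and construction script are empty, and some alternative instancing nodes sit disconnected.
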(event EventBeginPlay)

(event Collision|EventActorBeginOverlap
  (params (OtherActor :type Actor%20Object%20Reference)))

(event EventTick
  (params (DeltaSeconds :type Float%20%28single-precision%29)))

(event Input|KeyboardEvents|RightCtrl
  (params (Key :type Key%20Structure))
  (bind _nodos (Variables|Default|GetNodos))
  (:Pressed
    (Development|PrintText (Utilities|Text|ToText(Integer) (Utilities|Array|Length _nodos)))
    (for _array_element _nodos
      (Rendering|SetVisibility (Variables|/Script/NJVR.Nodo|GetNodoMesh _array_element) false false)
      (if (Variables|/Script/NJVR.Nodo|GetValid _array_element)
        (Components|InstancedStaticMesh|AddInstance (Variables|Default|GetNodosH) (Math|Transform|MakeTransform (.Location (Math|Transform|BreakTransform (Transformation|GetActorTransform _array_element))) (.Rotation (Math|Transform|BreakTransform (Transformation|GetActorTransform _array_element))) (* (.Scale (Math|Transform|BreakTransform (Transformation|GetActorTransform _array_element))) 1.5)))
        (else
          (Components|InstancedStaticMesh|AddInstance (Variables|Default|GetNodosVH) (Math|Transform|MakeTransform (.Location (Math|Transform|BreakTransform (Transformation|GetActorTransform _array_element))) (.Rotation (Math|Transform|BreakTransform (Transformation|GetActorTransform _array_element))) (.Scale (Math|Transform|BreakTransform (Transformation|GetActorTransform _array_element)))))))
      (Development|PrintText "Reemplazados"))
    (for _array_element_2 (Variables|Default|GetAristas)
      (bind _asarista_cilindro (Utilities|Casting|CastToAristaCilindro _array_element_2))
      (Rendering|SetVisibility (Variables|/Script/NJVR.AristaCilindro|GetAristaMesh _asarista_cilindro) false false)
      (Components|InstancedStaticMesh|AddInstance (Variables|Default|GetAristasH) (Transformation|GetActorTransform _asarista_cilindro)))))

(fn ConstructionScript)