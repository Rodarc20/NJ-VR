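; Debug test Blueprint for a semi-sphere VR visualization layout; as written, it only probes for objects along the world X axis.
; Each Tick, it line-traces one custom object channel from 1000 units toward negative X up to the actor's location.
; It draws the trace, cutting a second debug line at any impact point, and prints the hit actor's name.
; No layout logic is present.
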(event EventBeginPlay)

(event Collision|EventActorBeginOverlap
  (params (OtherActor :type Actor%20Object%20Reference)))

(event EventTick
  (params (DeltaSeconds :type Float%20%28single-precision%29))
  (bind _returnvalue (Transformation|GetActorLocation))
  (bind _returnvalue_2 (- _returnvalue "1000.000000, 0, 0"))
  (bind (_outhit _returnvalue_3) (Collision|LineTraceForObjects _returnvalue_2 _returnvalue (Utilities|Array|MakeArray "ObjectTypeQuery9") false 0 "ForOneFrame"))
  (Rendering|Debug|DrawDebugLine _returnvalue_2 (Math|Vector|SelectVector (.ImpactPoint (Collision|BreakHitResult _outhit)) _returnvalue _returnvalue_3) "(R=0.235000,G=0.000000,B=0.222407,A=1.000000)" 0.0 0.0)
  (if _returnvalue_3
    (Development|PrintText (Utilities|Text|ToText(String) (Utilities|GetObjectName (.HitActor (Collision|BreakHitResult _outhit)))) true true "(R=1.000000,G=0.328948,B=0.000000,A=1.000000)")))

(fn ConstructionScript)