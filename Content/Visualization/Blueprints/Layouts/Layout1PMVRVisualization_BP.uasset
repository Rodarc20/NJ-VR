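; VR node-visualization layout actor that lets the user scale, translate and rotate the visualization with motion controllers.
; Holding both grips records the starting controller distance, previews a temporary scale each Tick and commits it on release.
; Tick and Select input dispatch on visualization mode and task, driving laser node search or whole-visualization translation and rotation.
; Node and branch modes contain only empty task switches.
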(event EventBeginPlay)

(event Collision|EventActorBeginOverlap
  (params (OtherActor :type Actor%20Object%20Reference)))

(event EventTick
  (params (DeltaSeconds :type Float%20%28single-precision%29))
  ;[1 1 1] esto deberia estar dentro de una sola funcion
  (if (Variables|Default|GetbCalcularEscala)
    (Class|VRVisualization|CalcularEscalaTemporal)
    (Class|VRVisualization|AplicarEscala (Variables|Default|GetEscalaTemp)))
  (bind _returnvalue (Class|VRVisualization|GetVisualizationMode))
  ;[1 1 1] seleccionar el modo, sin area tengo 4, no selecciona es la visualizacion completa
  (switch Utilities|FlowControl|Switch|SwitchonEVRVisualizationMode _returnvalue
    (:EAll
      (Class|VRVisualization|BuscandoNodoConLaser))
    (:ENode
      ;[1 1 1] Nodo
      (bind _returnvalue_2 (Class|VRVisualization|GetVisualizationTask))
      ;;[1 1 1] la tarea seleccionar esta impicata en todos los otrso mdos, el ninguno deberia tener su propia funcion apra manipular laser apuntando e menu, no como esta ahora
      (switch Utilities|FlowControl|Switch|SwitchonEVRVisualizationTask _returnvalue_2))
    (:EBranch
      ;[1 1 1] Rama
      (bind _returnvalue_3 (Class|VRVisualization|GetVisualizationTask))
      (switch Utilities|FlowControl|Switch|SwitchonEVRVisualizationTask _returnvalue_3))
    (:ENoMode
      ;[1 1 1] Visualización, la tarea visualizacion solo deberia marcar dentro del menu
      (bind _returnvalue_4 (Class|VRVisualization|GetVisualizationTask))
      (switch Utilities|FlowControl|Switch|SwitchonEVRVisualizationTask _returnvalue_4
        (:ETraslationTask
          (if (Variables|Default|GetbNodoGuia)
            (Class|VRVisualization|TraslacionVisualizacion)
            (else
              (Class|VRVisualization|BuscandoNodoConLaser :!label _label))))
        (:ERotationTask
          (if (Variables|Default|GetRotar)
            (Class|VRVisualization|RotarVisualizacion)
            (goto _label)
            (else
              (goto _label))))
        (:EVisualizationTask
          (goto _label))
        (:ENoTask
          (goto _label))))))

(event Input|ActionEvents|InputActionSostenerDerecha
  (params (Key :type Key%20Structure))
  ;[0.055 0.055 0.055] Escala
  (:Pressed
    (Variables|Default|SetbGripDerecho true)
    (if (Variables|Default|GetbGripIzquierdo)
      (Variables|Default|SetbCalcularEscala true)
      (Variables|Default|SetDistanciaInicialControles (Math|Vector|VectorLength (- (Transformation|GetWorldLocation (Variables|Default|GetRightController)) (Transformation|GetWorldLocation (Variables|Default|GetLeftController)))))))
  (:Released
    (Variables|Default|SetbGripDerecho false)
    (Variables|Default|SetbCalcularEscala false)
    (bind _output_get (Variables|Default|SetEscala (Variables|Default|GetEscalaTemp)))
    (Class|VRVisualization|AplicarEscala _output_get)))

(event Input|ActionEvents|InputActionSostenerIzquierda
  (params (Key :type Key%20Structure))
  ;[0.055 0.055 0.055] Escala
  (:Pressed
    (Variables|Default|SetbGripIzquierdo true)
    (if (Variables|Default|GetbGripDerecho)
      (Variables|Default|SetbCalcularEscala true)
      (Variables|Default|SetDistanciaInicialControles (Math|Vector|VectorLength (- (Transformation|GetWorldLocation (Variables|Default|GetRightController)) (Transformation|GetWorldLocation (Variables|Default|GetLeftController)))))))
  (:Released
    (Variables|Default|SetbGripIzquierdo false)
    (Variables|Default|SetbCalcularEscala false)
    (bind _output_get (Variables|Default|SetEscala (Variables|Default|GetEscalaTemp)))
    (Class|VRVisualization|AplicarEscala _output_get)))

(event Input|ActionEvents|InputActionSelect
  (params (Key :type Key%20Structure))
  (:Pressed
    (bind _returnvalue (Class|VRVisualization|GetVisualizationMode))
    (switch Utilities|FlowControl|Switch|SwitchonEVRVisualizationMode _returnvalue
      (:EAll
        ;[1 1 1] Todo
        (bind _returnvalue_2 (Class|VRVisualization|GetVisualizationTask))
        (switch Utilities|FlowControl|Switch|SwitchonEVRVisualizationTask _returnvalue_2))
      (:ENode
        ;[1 1 1] Nodo
        (bind _returnvalue_3 (Class|VRVisualization|GetVisualizationTask))
        (switch Utilities|FlowControl|Switch|SwitchonEVRVisualizationTask _returnvalue_3))
      (:EBranch
        ;[1 1 1] Rama
        (bind _returnvalue_4 (Class|VRVisualization|GetVisualizationTask))
        (switch Utilities|FlowControl|Switch|SwitchonEVRVisualizationTask _returnvalue_4))
      (:ENoMode
        ;[1 1 1] Visualizacion
        (bind _returnvalue_5 (Class|VRVisualization|GetVisualizationTask))
        (switch Utilities|FlowControl|Switch|SwitchonEVRVisualizationTask _returnvalue_5
          (:ETraslationTask
            (Class|VRVisualization|TrasladarVisualizacionPressed))
          (:ERotationTask
            (Class|VRVisualization|RotarVisualizacionPressed))))))
  (:Released
    (bind _returnvalue_6 (Class|VRVisualization|GetVisualizationMode))
    (switch Utilities|FlowControl|Switch|SwitchonEVRVisualizationMode _returnvalue_6
      (:ENode
        ;[1 1 1] Nodo
        (bind _returnvalue_7 (Class|VRVisualization|GetVisualizationTask))
        (switch Utilities|FlowControl|Switch|SwitchonEVRVisualizationTask _returnvalue_7))
      (:EBranch
        ;[1 1 1] Rama
        (bind _returnvalue_8 (Class|VRVisualization|GetVisualizationTask))
        (switch Utilities|FlowControl|Switch|SwitchonEVRVisualizationTask _returnvalue_8))
      (:ENoMode
        ;[1 1 1] Visualizacion
        (bind _returnvalue_9 (Class|VRVisualization|GetVisualizationTask))
        (switch Utilities|FlowControl|Switch|SwitchonEVRVisualizationTask _returnvalue_9
          (:ETraslationTask
            (Class|VRVisualization|TrasladarVisualizacionReleased))
          (:ERotationTask
            (Class|VRVisualization|RotarVisualizacionReleased)))))))

(fn ConstructionScript)