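; NodoEsfera_BP is a node element for a visualization, with a NodoMesh and a Contenido widget.
; Its construction script makes a dynamic material instance from the mesh's first material and stores it in NodoMaterialDynamic for color changes.
; An unconnected VisualizarNodoPressed fragment would push ContenidoString to a ControlMenu2VR widget and print it, but never runs.
; The event graph has no active logic.
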(event EventBeginPlay)

(event Collision|EventActorBeginOverlap
  (params (OtherActor :type Actor%20Object%20Reference)))

(event EventTick
  (params (DeltaSeconds :type Float%20%28single-precision%29)))

(fn ConstructionScript
  (bind _nodomesh (Variables|Default|GetNodoMesh))
  ;[1 1 1] Creacion de la instancia dynamica del material, para poder hacer los cambios de color
  (bind _returnvalue (Rendering|Material|CreateDynamicMaterialInstance _nodomesh 0 (Utilities|Array|Get(acopy) (Rendering|Material|GetMaterials _nodomesh)) :!class /Script/Engine.PrimitiveComponent))
  (Variables|Default|SetNodoMaterialDynamic _returnvalue))